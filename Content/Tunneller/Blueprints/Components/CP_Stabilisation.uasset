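; CP_Stabilisation is an actor component that damps the motion of its physics-simulating owner for a limited time after play begins.
; On BeginPlay it gathers the owner's tagged shape components as stabilisers and starts a one-shot TTL timer that switches stabilisation off.
; While enabled and the root simulates physics, Tick applies a force at each stabiliser's location, opposing that shape's linear velocity and scaled by Stabilisation.
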(event Custom|Event%20Disable%20Stabilisation
  (Variables|Default|SetIsStabilisationEnabled false)
  (Development|PrintString (Utilities|String|BuildString(Object) "" "" self " Stabilisation Disabled")))

(event EventBeginPlay
  (bind _output_get (Variables|Default|SetOwner (Components|GetOwner)))
  (for _array_element (Actor|GetComponentsbyTag _output_get "/Script/Engine.ActorComponent" (Variables|Default|GetStabilisers%20Tag))
    (bind _asshape_component (Utilities|Casting|CastToShapeComponent _array_element))
    (Utilities|Array|Add (Variables|Default|GetStabilisers) _asshape_component)
    (Development|PrintString (Utilities|GetDisplayName _asshape_component)))
  (Utilities|Time|SetTimerbyEvent (delegate Custom|Event%20Disable%20Stabilisation) (Variables|Default|GetTTL)))

(event EventTick
  (params (DeltaSeconds :type Float%20%28single-precision%29))
  (if (and (Variables|Default|GetIsStabilisationEnabled) (Physics|IsSimulatingPhysics (Variables|/Script/Engine.Actor|GetRootComponent (Variables|Default|GetOwner)) "None"))
    (for _array_element (Variables|Default|GetStabilisers)
      (bind _output_get (Variables|Default|SetShape _array_element))
      (bind _returnvalue (Physics|GetPhysicsLinearVelocity _output_get "None"))
      (Class|PrimitiveComponent|AddForceatLocation (Variables|Default|GetShape) (* _returnvalue (Variables|Default|GetStabilisation) -1.0) (Transformation|GetWorldLocation (Variables|Default|GetShape)) "None"))))