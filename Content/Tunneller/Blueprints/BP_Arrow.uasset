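; BP_Arrow is an arrow projectile launched by a forward physics impulse that sticks into and damages what it hits.
; On overlap, it line-traces the touched component along the body's length to find hit point, normal and bone.
; Hits with a named bone and steep enough angle disable collision and physics, attach to that bone, embed the arrow, and apply damage if an instigator exists.
; Debug prints and arrows visualise impacts.
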(event OnComponentBeginOverlap(Body)
  (params (OverlappedComponent :type Primitive%20Component%20Object%20Reference) (OtherActor :type Actor%20Object%20Reference) (OtherComp :type Primitive%20Component%20Object%20Reference) (OtherBodyIndex :type Integer) (bFromSweep :type Boolean) (SweepResult :type Hit%20Result%20Structure%20%28by%20ref%29))
  (bind _returnvalue (Transformation|GetActorLocation))
  (bind _instigator (Variables|Actor|GetInstigator))
  (bind _body (Variables|Default|GetBody))
  (bind _returnvalue_2 (Transformation|GetWorldLocation _body))
  (bind _returnvalue_3 (Math|Vector|GetForwardVector _body))
  (bind (_min _max) (Components|StaticMesh|GetLocalBounds _body))
  (Variables|Default|SetTarget%20Actor OtherActor)
  (bind _output_get (Variables|Default|SetTarget%20Component OtherComp))
  ;[1 1 1] Line Trace
  (bind (_hitlocation _hitnormal _bonename) (Collision|LineTraceComponent _output_get (+ _returnvalue_2 (* _returnvalue_3 (.x _min))) (+ _returnvalue_2 (* _returnvalue_3 (.x _max))) false true true))
  (Variables|Default|SetHit%20Location _hitlocation)
  (Variables|Default|SetHit%20Normal _hitnormal)
  (Variables|Default|SetTarget%20Bone _bonename)
  ;[1 1 1] Do not attach condition
  (if (or (== (Variables|Default|GetTarget%20Bone) "") (< (Math|Float|Absolute(Float) (Math|Vector|DotProduct (Variables|Default|GetHit%20Normal) (Transformation|GetActorForwardVector))) 0.5))
    _
    (else
      ;[1 1 1] Attach
      (Collision|SetActorEnableCollision false)
      (Physics|SetSimulatePhysics (Variables|Default|GetBody) false)
      (Transformation|AttachComponentToComponent (Variables|Default|GetTarget%20Component) (Variables|Default|GetTarget%20Bone) "KeepWorld" "KeepWorld" "KeepWorld" true)
      ;[1 1 1] Penetration Depth
      (Transformation|SetActorLocation (+ (Variables|Default|GetHit%20Location) (* (Transformation|GetActorForwardVector) 1e+01)) false false)
      ;[1 1 1] Damage
      (Utilities|IsValid _instigator
        (:Is%20Valid
          (Game|Damage|ApplyDamage (Variables|Default|GetTarget%20Actor) 1e+01 (Pawn|GetController _instigator) self)))))
  ;[1 1 1] Debug
  (Development|PrintString (Utilities|String|BuildString(Name) "attached to " (Utilities|GetDisplayName (Variables|Default|GetTarget%20Component)) (Variables|Default|GetTarget%20Bone) ""))
  (Rendering|Debug|DrawDebugArrow (Variables|Default|GetHit%20Location) (+ (Variables|Default|GetHit%20Location) (* (Variables|Default|GetHit%20Normal) 1e+01)) 1.0 "(R=0.000000,G=1.000000,B=0.387439,A=1.000000)" 1e+03 1.0)
  (Rendering|Debug|DrawDebugArrow _returnvalue (+ _returnvalue (* (Transformation|GetActorForwardVector) 1e+01)) 1.0 "(R=1.000000,G=0.739390,B=0.000000,A=1.000000)" 1e+03 1.0))

(event EventBeginPlay
  (Physics|AddImpulse (Variables|Default|GetBody) (* (Variables|Default|GetImpulse) (Transformation|GetActorForwardVector)) "None" false))

(fn ConstructionScript)