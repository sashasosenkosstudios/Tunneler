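; BP_Bow is a pickup weapon that fires projectiles when used.
; Pickup sets the new holder as owner and instigator, then disables the pickup area's collision.
; Use spawns the projectile class at the ProjectileSpawn transform, owned by the bow and carrying its instigator.
; If a projectile movement component exists, its velocity becomes a fixed-speed shot randomized within a forward cone, plus the holder's velocity.
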(event EventUse
  (bind _returnvalue (Game|SpawnActorfromClass (Variables|Default|GetProjectile) (Transformation|GetWorldTransform (Variables|Default|GetProjectile%20Spawn)) "Undefined" self (Game|GetInstigator)))
  (Utilities|IsValid (Actor|GetComponentbyClass _returnvalue "/Script/Engine.ProjectileMovementComponent")
    (:Is%20Valid
      (Variables|/Script/Engine.MovementComponent|SetVelocity (Actor|GetComponentbyClass _returnvalue "/Script/Engine.ProjectileMovementComponent") (+ (Transformation|GetVelocity (Components|GetOwner)) (* (Math|Random|RandomUnitVectorinConeinDegrees (Transformation|GetActorForwardVector _returnvalue) 1e+01) 2e+03))))))

(event EventPickup
  (params (Owner :type Pawn%20Object%20Reference))
  (bind _output_get (Variables|Actor|SetInstigator Owner))
  (Actor|SetOwner _output_get)
  (Collision|SetCollisionEnabled (Variables|Default|GetPickup%20Area) "NoCollision"))

(fn ConstructionScript)