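; BP_CinematicArrow is an arrow projectile, named for cinematic use, that damages and sticks into what it overlaps.
; On Body overlap it halts projectile movement and, if its Instigator is valid, applies fixed damage, disables further overlaps and physics, and attaches to the hit component's bone, keeping world transform.
; When projectile movement stops, Body switches to physics simulation with overlaps disabled.
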(event OnComponentBeginOverlap(Body)
  (params (OverlappedComponent :type Primitive%20Component%20Object%20Reference) (OtherActor :type Actor%20Object%20Reference) (OtherComp :type Primitive%20Component%20Object%20Reference) (OtherBodyIndex :type Integer) (bFromSweep :type Boolean) (SweepResult :type Hit%20Result%20Structure%20%28by%20ref%29))
  (bind _instigator (Variables|Actor|GetInstigator))
  (Variables|/Script/Engine.ProjectileMovementComponent|SetbSimulationEnabled (Variables|Default|GetProjectileMovement) false)
  (Variables|Default|SetTarget%20Actor OtherActor)
  (Variables|Components|SetTarget%20Component OtherComp)
  (Variables|Default|SetTarget%20Bone (.hitbonename SweepResult))
  (Development|PrintString (Utilities|GetDisplayName 0))
  (Utilities|IsValid _instigator
    (:Is%20Valid
      (Game|Damage|ApplyDamage (Variables|Default|GetTarget%20Actor) 5e+01 (Pawn|GetController _instigator) self)
      (Variables|/Script/Engine.PrimitiveComponent|SetbGenerateOverlapEvents (Variables|Default|GetBody) false)
      (Physics|SetSimulatePhysics (Variables|Default|GetBody) false)
      (Transformation|AttachComponentToComponent (Variables|Components|GetTarget%20Component) (Variables|Default|GetTarget%20Bone) "KeepWorld" "KeepWorld" "KeepWorld" true)
      (Development|PrintString (Utilities|String|BuildString(Name) "attached to " (Utilities|GetDisplayName (Variables|Components|GetTarget%20Component)) (Variables|Default|GetTarget%20Bone) "")))))

(event OnProjectileStop(ProjectileMovement)
  (params (ImpactResult :type Hit%20Result%20Structure%20%28by%20ref%29))
  (Physics|SetSimulatePhysics (Variables|Default|GetBody) true)
  (Variables|/Script/Engine.PrimitiveComponent|SetbGenerateOverlapEvents (Variables|Default|GetBody) false))

(fn ConstructionScript)